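; Behavior tree task that makes an NPC attack the enemy stored in the CurrentEnemy blackboard key.
; It snaps the NPC's yaw toward the enemy via RotateTowards, whose parameter names are swapped, and raises IsAttackingAnim.
; In primary range it calls NPCAttack and succeeds after the cooldown divided by animation rate; otherwise it fails immediately.
; The animation flag clears after either result.
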(event `self.ReceiveExecuteAI`
  (params (OwnerController :type "AIController Object Reference") (ControlledPawn :type "Pawn Object Reference"))
  (bind _returnvalue (`BTFunctionLibrary.GetBlackboardValueAsActor` (`self.CurrentEnemy`)))
  (bind _ascharacter_npc_master (cast `/Game/BluePrints/Character_NPC_master` ControlledPawn))
  (`self.RotateTowards` _returnvalue _ascharacter_npc_master)
  (set `/Game/BluePrints/Character_NPC_master.isAttackingAnim?` true _ascharacter_npc_master)
  (if (<= (`Actor.GetDistanceTo` _ascharacter_npc_master _returnvalue) (`/Game/BluePrints/Character_NPC_master.PrimaryAttackRange` _ascharacter_npc_master))
    (`/Game/BluePrints/Character_NPC_master.NPCAttack` _ascharacter_npc_master _returnvalue)
    (`KismetSystemLibrary.Delay` (/ (`/Game/BluePrints/Character_NPC_master.PrimaryAttackCooldownTime` _ascharacter_npc_master) (`/Game/BluePrints/Character_NPC_master.PrimaryAttackAnimRate` _ascharacter_npc_master)))
    (`self.FinishExecute` true)
    (else
      (`self.FinishExecute` false)))
  (set `/Game/BluePrints/Character_NPC_master.isAttackingAnim?` false _ascharacter_npc_master))

(fn `RotateTowards`
  (params (`Actor To Rotate` :type "Actor Object Reference") (`Look At` :type "Actor Object Reference"))
  (`SceneComponent.K2_SetWorldRotation` (`Actor.RootComponent` `Look At`) (`KismetMathLibrary.MakeRotator` 0.0 0.0 (.yaw (`KismetMathLibrary.FindLookAtRotation` (`Actor.K2_GetActorLocation` `Look At`) (`Actor.K2_GetActorLocation` `Actor To Rotate`)))) false false))