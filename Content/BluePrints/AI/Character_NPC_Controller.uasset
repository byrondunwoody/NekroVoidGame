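; AI controller for NPCs that runs a friendly or aggressive behavior tree on a shared blackboard, based on the pawn's behaviour.
; AI Perception sets UnderAttack on attack or death tags; otherwise, sensing a living other-faction NPC alerts friendlies or gives hostiles an enemy via SetEnemy.
; A pause function toggles blackboard activity for player interaction.
; Losing a target only prints for hostiles, and much older enemy-list and player-detection logic is disconnected.
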(event `self.ReceiveBeginPlay`
  (bind _controlledpawn (`self.ControlledPawn`))
  (bind _ascharacter_npc_master (cast `/Game/BluePrints/Character_NPC_master` (`self.K2_GetPawn`)))
  (set `self.ControlledPawn` _ascharacter_npc_master)
  (`|ExecutionSequence`
    (:`then_0`
      (switch `/Game/BluePrints/AI/NPCBehaviourTypes` (`/Game/BluePrints/Character_NPC_master.NPCBehaviour` _controlledpawn)
        (:`NewEnumerator0`
          (`self.UseBlackboard` "/Game/BluePrints/AI/CharacterNPC-BB.CharacterNPC-BB")
          (`self.RunBehaviorTree` "/Game/BluePrints/AI/CharacterNPCFriendly-BT.CharacterNPCFriendly-BT")
          (`KismetSystemLibrary.PrintString` (`KismetStringLibrary.Concat_StrStr` (`KismetSystemLibrary.GetDisplayName` (`self.ControlledPawn`)) " - Friendly AI Activated") true true (struct :`R` 0.107088 :`G` 1.0 :`A` 1.0)))
        (:`NewEnumerator2`
          (`self.UseBlackboard` "/Game/BluePrints/AI/CharacterNPC-BB.CharacterNPC-BB")
          (`self.RunBehaviorTree` "/Game/BluePrints/AI/CharacterNPCAggressive-BT.CharacterNPCAggressive-BT")
          (`KismetSystemLibrary.PrintString` "Hostile AI Activated" true true (struct :`R` 1.0 :`B` 0.069441 :`A` 1.0)))))
    (:`then_1`
      (switch `/Game/BluePrints/AI/NPCActivityTypes` (`/Game/BluePrints/Character_NPC_master.NPCActivity` _controlledpawn)))))

(event `self.PawnSensing.OnSeePawn`
  (params (Pawn :type "Pawn Object Reference")))

(event `self.AIPerception.OnTargetPerceptionUpdated`
  (params (Actor :type "Actor Object Reference") (Stimulus :type "AIStimulus Structure"))
  (bind (_age _expirationage _strength _stimuluslocation _receiverlocation _tag _bsuccessfullysensed) (break `AIStimulus` Stimulus))
  (bind _controlledpawn (`self.ControlledPawn`))
  (if (`/Game/BluePrints/Character_NPC_master.AIEnabled?` (`self.ControlledPawn`))
    (if true
      ;[1 0.9044 0] DEBUG- NOT SPECTATOR PAWN
      (if (!= (`GameplayStatics.GetObjectClass` Actor) "/Script/Engine.SpectatorPawn")
        (set `self.SensedActor` Actor)
        (set `self.SensedActorLocation` _stimuluslocation)
        ;[1 0 0] SENSED?
        (set `self.SuccessfullySensed?` _bsuccessfullysensed)
        ;[0.3375 0.4114 1] REACTONS FOR DIFFERENT EVENTS
        (switch `name` _tag
          (:`Default`
            (if _bsuccessfullysensed
              ;[1 1 1] NPC set as enemy
              (bind _ascharacter_npc_master (cast `/Game/BluePrints/Character_NPC_master` (`self.SensedActor`)))
              (if (and (`|EnumInequality` (`/Game/BluePrints/Character_NPC_master.NPCFaction` _ascharacter_npc_master) (`/Game/BluePrints/Character_NPC_master.NPCFaction` (`self.ControlledPawn`))) (not (`/Game/BluePrints/Character_NPC_master.isDead?` _ascharacter_npc_master)))
                (switch `/Game/BluePrints/AI/NPCBehaviourTypes` (`/Game/BluePrints/Character_NPC_master.NPCBehaviour` (`self.ControlledPawn`))
                  (:`NewEnumerator0`
                    (set `/Game/BluePrints/Character_NPC_master.NPCActivity` "NewEnumerator7" (`self.ControlledPawn`)))
                  (:`NewEnumerator2`
                    (`self.SetEnemy` (`self.SensedActor`) true (`self.SensedActorLocation`))
                    (set `self.HaveAnEnemy?` true))))
              (else
                (switch `/Game/BluePrints/AI/NPCBehaviourTypes` (`/Game/BluePrints/Character_NPC_master.NPCBehaviour` (`self.ControlledPawn`))
                  (:`NewEnumerator2`
                    (`KismetSystemLibrary.PrintString` "LOST ENEMY" true true (struct :`R` 1.0 :`B` 0.140206 :`A` 1.0)))))))
          (:`NPCDEATH`
            ;[1 1 1] If Attack or Death Noise event is detected
            (set `/Game/BluePrints/Character_NPC_master.NPCActivity` "NewEnumerator7" _controlledpawn :!label _label)
            (`KismetSystemLibrary.PrintString` (`KismetStringLibrary.Concat_StrStr` (`KismetSystemLibrary.GetDisplayName` _controlledpawn) "UNDER ATTACK TAG") true true (struct :`R` 1.0 :`G` 0.860183 :`B` 0.074322 :`A` 1.0)))
          (:`NPCATTACK`
            (goto _label)))))))

(event `self.AIPerception.OnPerceptionUpdated`
  (params (UpdatedActors :type "Array of Actor Object Reference"))
  ;[0.7542 1 0.7803] Broken
)

(fn `AISetActivityPausedState`
  (params (Paused :type Boolean))
  (locals (NPCStoredActicityState :type "/Game/BluePrints/AI/NPCActivityTypes Enum"))
  (bind _returnvalue (`AIBlueprintHelperLibrary.GetBlackboard` (`self.ControlledPawn`)))
  (if Paused
    (bind _output_get (set `local.NPCStoredActicityState` "NewEnumerator0"))
    (`BlackboardComponent.SetValueAsEnum` _returnvalue (`self.BBNPCActivity`) _output_get)
    (`BlackboardComponent.SetValueAsBool` _returnvalue (`self.BBInteractingPlayer?`) true)
    (`KismetSystemLibrary.PrintString` "SET AI PAUSED STATE")
    (else
      (`BlackboardComponent.SetValueAsBool` (`AIBlueprintHelperLibrary.GetBlackboard` (`self.ControlledPawn`)) (`self.BBInteractingPlayer?`) false)
      (`BlackboardComponent.SetValueAsEnum` (`AIBlueprintHelperLibrary.GetBlackboard` (`self.ControlledPawn`)) (`self.BBNPCActivity`) (`self.NPCsActivityType`))
      (`KismetSystemLibrary.PrintString` "SET AI PAUSED STATE: RETURNED"))))

(fn `OnRep_BBHaveEnemy?`)

(fn `SetEnemy`
  (params (`New Enemy` :type "Actor Object Reference") (`SuccessfullySensed?` :type Boolean) (EnemyLocation :type "Vector Structure"))
  (`BlackboardComponent.SetValueAsVector` (`AIBlueprintHelperLibrary.GetBlackboard` (`self.ControlledPawn`)) (`self.BBLastSeenEnemyLocation`) EnemyLocation)
  (if `SuccessfullySensed?`
    (`BlackboardComponent.SetValueAsObject` (`AIBlueprintHelperLibrary.GetBlackboard` (`self.ControlledPawn`)) (`self.BBEnemy`) `New Enemy`)
    (set `/Game/BluePrints/Character_NPC_master.CurrentEnemy` `New Enemy` (`self.ControlledPawn`))
    (`BlackboardComponent.SetValueAsBool` (`AIBlueprintHelperLibrary.GetBlackboard` (`self.ControlledPawn`)) (`self.BBHaveEnemy?`) true)
    (return)))

(fn `UserConstructionScript`)