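; NPC route point actor that links to following points through its NextPoint array, forming a route graph visualized with debug lines.
; The construction script draws lines from its Point component to every linked point's Point, repeating the full set for each valid entry via a nested loop.
; Invalid entries print a "No Valid Goal" warning, while the inner loop does not check validity.
; The event graph holds no runtime logic.
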(fn `UserConstructionScript`
  (for _array_element (`self.NextPoint`)
    (if (`KismetSystemLibrary.IsValid` _array_element)
      (for _array_element_2 (`self.NextPoint`)
        (`KismetSystemLibrary.DrawDebugLine` (`SceneComponent.K2_GetComponentLocation` (`self.point`)) (`SceneComponent.K2_GetComponentLocation` (`/Game/BluePrints/AI/NPCRoutePoint.point` _array_element_2)) (struct :`R` 1.0 :`B` 0.536849 :`A` 1.0) -1.0 6.0))
      (else
        (`KismetSystemLibrary.PrintString` "No Valid Goal")))))