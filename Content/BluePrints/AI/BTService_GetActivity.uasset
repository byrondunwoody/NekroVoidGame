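; Behavior tree service that copies an NPC's current activity into the blackboard for its AI.
; On each tick it casts the AI controller's pawn to Character_NPC_master and writes its NPCActivity enum to the NPCActivityKey entry.
; A failed cast only prints a debug message, and an unconnected debug print of the activity remains in the graph.
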(event `self.ReceiveActivation`
  (params (OwnerActor :type "Actor Object Reference"))
  ;[1 1 1] Begin Player bscly
)

(event `self.ReceiveTick`
  (params (OwnerActor :type "Actor Object Reference") (DeltaSeconds :type "Float (single-precision)"))
  ;[1 1 1] Always use this
  (bind _ascharacter_npc_master (cast `/Game/BluePrints/Character_NPC_master` (`Controller.K2_GetPawn` (`AIBlueprintHelperLibrary.GetAIController` OwnerActor)))
    (:`then`
      (`BTFunctionLibrary.SetBlackboardValueAsEnum` (`self.NPCActivityKey`) (`/Game/BluePrints/Character_NPC_master.NPCActivity` _ascharacter_npc_master)))
    (:`CastFailed`
      (`KismetSystemLibrary.PrintString` "Cast Failerd"))))