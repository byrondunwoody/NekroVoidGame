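; Behavior tree task that copies an NPC's current enemy into the blackboard.
; On execute it casts the controlled pawn to Character_NPC_master and checks whether its CurrentEnemy is valid.
; A valid enemy is written to the enemy object key, the have-enemy flag is set true and the task succeeds.
; With no valid enemy the task fails and leaves both keys unchanged.
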(event `self.ReceiveExecuteAI`
  (params (OwnerController :type "AIController Object Reference") (ControlledPawn :type "Pawn Object Reference"))
  (bind _ascharacter_npc_master (cast `/Game/BluePrints/Character_NPC_master` ControlledPawn))
  (bind _currentenemy (`/Game/BluePrints/Character_NPC_master.CurrentEnemy` _ascharacter_npc_master))
  (if (`KismetSystemLibrary.IsValid` _currentenemy)
    (`|ExecutionSequence`
      (:`then_0`
        (`BTFunctionLibrary.SetBlackboardValueAsObject` (`self.NPCCurrentEnemy`) _currentenemy))
      (:`then_1`
        (`BTFunctionLibrary.SetBlackboardValueAsBool` (`self.NPCHaveEnemy`) true))
      (:`then_2`
        (`self.FinishExecute` true)))
    (else
      (`self.FinishExecute` false))))