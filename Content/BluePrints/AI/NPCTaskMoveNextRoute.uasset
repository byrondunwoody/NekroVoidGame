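; Behavior tree task that walks an NPC along a branching route of linked waypoints.
; It moves the Character_NPC_master pawn to its current route goal with a randomized acceptance radius.
; On success it picks a random NextPoint, using a decremented array length, stores it on the NPC and in the blackboard, then finishes.
; A failed cast or move never finishes the task.
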(event `self.ReceiveExecuteAI`
  (params (OwnerController :type "AIController Object Reference") (ControlledPawn :type "Pawn Object Reference"))
  (bind _ascharacter_npc_master (cast `/Game/BluePrints/Character_NPC_master` ControlledPawn))
  (bind _npcroutecurrentgoal (`/Game/BluePrints/Character_NPC_master.NPCRouteCurrentGoal` _ascharacter_npc_master))
  (`|AIMoveTo` _ascharacter_npc_master (0.0 0.0 0.0) _npcroutecurrentgoal (`KismetMathLibrary.RandomFloatInRange` 0.0 (`self.randomAcceptanceRadius`))
    (:`OnSuccess`
      (bind _nextpoint (`/Game/BluePrints/AI/NPCRoutePoint.NextPoint` _npcroutecurrentgoal))
      (bind _result (`/Engine/EditorBlueprintResources/StandardMacros.DecrementInt` (`KismetArrayLibrary.Array_Length` _nextpoint))
        (:`  `
          (bind _output_get (set `/Game/BluePrints/Character_NPC_master.NPCRouteCurrentGoal` (`|GetArrayItem` _nextpoint (`KismetMathLibrary.RandomInteger` _result)) _ascharacter_npc_master))
          (`BTFunctionLibrary.SetBlackboardValueAsObject` (`self.NPCRoutePointKey`) _output_get)
          (`self.FinishExecute` true))))))