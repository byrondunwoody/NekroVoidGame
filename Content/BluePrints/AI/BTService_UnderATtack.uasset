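; Behavior tree service that sets up fleeing when an NPC is under attack.
; On activation, it copies the NPC's AttackingPawn to the blackboard and writes a flee location; Tick is empty.
; A valid attacker yields a direction away from it with random ±45° yaw, scaled by FleeRange without adding the NPC's position.
; Otherwise, it picks a random navigable point within FleeRange of the NPC.
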(event `self.ReceiveTick`
  (params (OwnerActor :type "Actor Object Reference") (DeltaSeconds :type "Float (single-precision)")))

(event `self.ReceiveActivation`
  (params (OwnerActor :type "Actor Object Reference"))
  (bind _returnvalue (`Controller.K2_GetPawn` (`AIBlueprintHelperLibrary.GetAIController` OwnerActor)))
  ;[1 1 1] Always use this
  (bind _ascharacter_npc_master (cast `/Game/BluePrints/Character_NPC_master` _returnvalue))
  (bind _attackingpawn (`/Game/BluePrints/Character_NPC_master.AttackingPawn` _ascharacter_npc_master))
  (`BTFunctionLibrary.SetBlackboardValueAsObject` (`self.BBAttackingPawn`) _attackingpawn)
  ;[1 1 1] If the attacking pawn(TRUE) was set or NPC heard it(FALSE)
  (if (`KismetSystemLibrary.IsValid` _attackingpawn)
    (`BTFunctionLibrary.SetBlackboardValueAsVector` (`self.BBFleeLocation`) (* (`KismetMathLibrary.GetForwardVector` (`KismetMathLibrary.MakeRotator` (.roll (`KismetMathLibrary.FindLookAtRotation` (`Actor.K2_GetActorLocation` _attackingpawn) (`Actor.K2_GetActorLocation` OwnerActor))) (.pitch (`KismetMathLibrary.FindLookAtRotation` (`Actor.K2_GetActorLocation` _attackingpawn) (`Actor.K2_GetActorLocation` OwnerActor))) (+ (.yaw (`KismetMathLibrary.FindLookAtRotation` (`Actor.K2_GetActorLocation` _attackingpawn) (`Actor.K2_GetActorLocation` OwnerActor))) (`KismetMathLibrary.RandomFloatInRange` -45.0 45.0)))) (`self.FleeRange`)))
    (else
      (`BTFunctionLibrary.SetBlackboardValueAsVector` (`self.BBFleeLocation`) (`NavigationSystem.K2_GetRandomLocationInNavigableRadius` (`Actor.K2_GetActorLocation` _returnvalue) (`self.FleeRange`))))))