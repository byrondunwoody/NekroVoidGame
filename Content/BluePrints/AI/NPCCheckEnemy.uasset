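; Behavior tree task that validates an NPC's current enemy stored in the blackboard.
; An invalid target clears the enemy keys and fails the task, while the player always passes without a death check.
; NPC targets also succeed, clearing the keys first if the enemy is dead.
; Logic for picking a replacement from the NPC's enemy list and updating its controller is present but disconnected.
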(event `self.ReceiveExecuteAI`
  (params (OwnerController :type "AIController Object Reference") (ControlledPawn :type "Pawn Object Reference"))
  (bind _returnvalue (`BTFunctionLibrary.GetBlackboardValueAsActor` (`self.NPCCurrentEnemy`)))
  (if (`KismetSystemLibrary.IsValid` _returnvalue)
    ;[1 1 1] Is it the player?
    (if (== _returnvalue (`GameplayStatics.GetPlayerPawn` 0))
      (`self.FinishExecute` true)
      (else
        (bind _ascharacter_npc_master (cast `/Game/BluePrints/Character_NPC_master` ControlledPawn))
        (set `self.ControlledNpcPawn` _ascharacter_npc_master)
        (bind _ascharacter_npc_master_2 (cast `/Game/BluePrints/Character_NPC_master` (`BTFunctionLibrary.GetBlackboardValueAsActor` (`self.NPCCurrentEnemy`))))
        (set `self.CheckedEnemy` _ascharacter_npc_master_2)
        ;[1 0 0.06761] ENEMY IS DEAD
        (if (`/Game/BluePrints/Character_NPC_master.isDead?` (`self.CheckedEnemy`))
          ;[1 1 1] Clear Black Board value
          (`BTFunctionLibrary.SetBlackboardValueAsObject` (`self.NPCCurrentEnemy`))
          (`BTFunctionLibrary.SetBlackboardValueAsBool` (`self.NPCHaveEnemy`))
          (`self.FinishExecute` true)
          (else
            (`self.FinishExecute` true)))))
    (else
      ;[1 1 1] If not valid , have to reset everything
      (`BTFunctionLibrary.SetBlackboardValueAsObject` (`self.NPCCurrentEnemy`))
      (`BTFunctionLibrary.SetBlackboardValueAsBool` (`self.NPCHaveEnemy`))
      (`self.FinishExecute` false))))

(fn `AIControllerSetNeedNewEnemy`
  (params (`NeedNewEnemy?` :type Boolean))
  (bind _ascharacter_npc_controller (cast `/Game/BluePrints/AI/Character_NPC_Controller` (`Pawn.GetController` (`self.ControlledNpcPawn`))))
  (set `/Game/BluePrints/AI/Character_NPC_Controller.HaveAnEnemy?` `NeedNewEnemy?` _ascharacter_npc_controller)
  (return))