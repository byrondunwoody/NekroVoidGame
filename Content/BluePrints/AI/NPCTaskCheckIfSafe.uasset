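; Behavior tree task that checks whether an NPC has other-faction NPCs within its safety distance.
; It runs a debug-drawn sphere trace at the pawn and compares factions with hits whose class is exactly Character_NPC_master.
; Each differing faction only prints "not safe", while each match resets the NPC's activity, and the task then finishes successfully.
; Author comments mark the comparison as faulty and restoring the previous activity as unfinished.
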(event `self.ReceiveExecuteAI`
  (params (OwnerController :type "AIController Object Reference") (ControlledPawn :type "Pawn Object Reference"))
  (bind _returnvalue (`Actor.K2_GetActorLocation` ControlledPawn))
  (bind _ascharacter_npc_master (cast `/Game/BluePrints/Character_NPC_master` ControlledPawn))
  (set `self.ComparingFaction` (`/Game/BluePrints/Character_NPC_master.NPCFaction` _ascharacter_npc_master))
  (bind _outhits (`KismetSystemLibrary.SphereTraceMulti` :`Start` _returnvalue :`End` _returnvalue :`Radius` (`self.NPCSafetyDistance`) :`TraceChannel` "TraceTypeQuery1" :`DrawDebugType` "ForDuration"))
  (for _array_element _outhits
    (bind (_bblockinghit _binitialoverlap _time _location _impactpoint _normal _impactnormal _physmat _hitactor) (`GameplayStatics.BreakHitResult` _array_element))
    (if (== (`GameplayStatics.GetObjectClass` _hitactor) "/Game/BluePrints/Character_NPC_master.Character_NPC_master_C")
      (bind _ascharacter_npc_master_2 (cast `/Game/BluePrints/Character_NPC_master` _hitactor))
      ;[1 0 0] SOMETHING IS WRONG HERE - always return flase
      (if (`|EnumInequality` (`/Game/BluePrints/Character_NPC_master.NPCFaction` _ascharacter_npc_master_2) (`self.ComparingFaction`))
        (`KismetSystemLibrary.PrintString` "ITS NOT SAFE" true true (struct :`R` 1.0 :`B` 0.738211 :`A` 1.0))
        (else
          (`KismetSystemLibrary.PrintString` "IT IS SAFE" true true (struct :`G` 0.317408 :`B` 1.0 :`A` 1.0))
          ;[1 1 1] Needs to go back to last activity it was doing
          (set `/Game/BluePrints/Character_NPC_master.NPCActivity` "NewEnumerator0" _ascharacter_npc_master)))))
  (`self.FinishExecute` true))